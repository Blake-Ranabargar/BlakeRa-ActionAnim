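; BP_WallButton is a wall button that makes the Blake sandbox character reach its right hand toward it when nearby.
; On sphere overlap, it passes the button's world location to the character's animation blueprint as the right-hand IK target.
; A timeline blends the IK alpha in, and reverses when any overlap ends.
; It contains no press or activation logic.
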(event OnComponentBeginOverlap(Sphere_Col)
  (params (OverlappedComponent :type Primitive%20Component%20Object%20Reference) (OtherActor :type Actor%20Object%20Reference) (OtherComp :type Primitive%20Component%20Object%20Reference) (OtherBodyIndex :type Integer) (bFromSweep :type Boolean) (SweepResult :type Hit%20Result%20Structure%20%28by%20ref%29))
  (bind _assandbox_character_cmc_blake (Utilities|Casting|CastToSandboxCharacter_CMC_Blake OtherActor))
  (bind _assandbox_character_cmc_abp_blake (Utilities|Casting|CastToSandboxCharacter_CMC_ABP_Blake (Components|SkeletalMesh|GetAnimInstance (Variables|/Script/Engine.Character|GetMesh _assandbox_character_cmc_blake))))
  (Variables|Default|SetABP _assandbox_character_cmc_abp_blake)
  (Variables|/Game/Blake/SandboxCharacter_CMC_ABP_Blake.SandboxCharacter_CMC_ABP_Blake_C|SetRight_Hand_IK_Target (Variables|Default|GetABP) (Transformation|GetWorldLocation (Variables|Default|GetButton)))
  (bind _to_button (Timeline|TL_To_Button Play)
    (:Update
      (Variables|/Game/Blake/SandboxCharacter_CMC_ABP_Blake.SandboxCharacter_CMC_ABP_Blake_C|SetRight_Hand_IK_Alpha (Variables|Default|GetABP) _to_button))))

(event OnComponentEndOverlap(Sphere_Col)
  (params (OverlappedComponent :type Primitive%20Component%20Object%20Reference) (OtherActor :type Actor%20Object%20Reference) (OtherComp :type Primitive%20Component%20Object%20Reference) (OtherBodyIndex :type Integer))
  (bind _to_button (Timeline|TL_To_Button Reverse)
    (:Update
      (Variables|/Game/Blake/SandboxCharacter_CMC_ABP_Blake.SandboxCharacter_CMC_ABP_Blake_C|SetRight_Hand_IK_Alpha (Variables|Default|GetABP) _to_button))))

(event EventBeginPlay)

(event Collision|EventActorBeginOverlap
  (params (OtherActor :type Actor%20Object%20Reference)))

(event EventTick
  (params (DeltaSeconds :type Float%20%28single-precision%29)))

(fn ConstructionScript)